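; Tuna food ingredient pickup that the player collects by pressing F while standing inside its Box volume.
; The actor enables input from player controller 0 on BeginPlay, so it handles the key press itself.
; On F, it checks that the player pawn overlaps the Box, casts it to BP_MainChara, calls AjoutPoisson to add fish, then destroys itself.
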(event EventBeginPlay
  ;[0.15 0.15 0.15 0.5] Keyboard qui marche
  (Input|EnableInput (Game|GetPlayerController 0)))

(event Input|KeyboardEvents|F
  (params (Key :type Key%20Structure :default "None"))
  ;[0.15 0.15 0.15 0.5] Presser F pour détruire plats
  (:Pressed
    (if (Collision|IsOverlappingActor (Variables|Default|Get%20box) (Game|Player|GetPlayerPawn 0) :!class /Script/Engine.PrimitiveComponent)
      (bind _asbp_main_chara (Utilities|Casting|CastToBP_MainChara (Game|Player|GetPlayerPawn 0)))
      (Default|AjoutPoisson _asbp_main_chara)
      (Actor|DestroyActor))))

(fn ConstructionScript)