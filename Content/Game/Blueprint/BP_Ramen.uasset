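; BP_Ramen is a pickup dish that the player collects with the F key.
; It enables input on BeginPlay, and pressing F while the player pawn overlaps its Box calls AjoutPlat on BP_MainChara, then destroys the actor.
; Box begin and end overlap events show and hide the TexteF prompt, without filtering which actor overlaps.
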(event OnComponentBeginOverlap(Box)
  (params (OverlappedComponent :type Primitive%20Component%20Object%20Reference) (OtherActor :type Actor%20Object%20Reference) (OtherComp :type Primitive%20Component%20Object%20Reference) (OtherBodyIndex :type Integer) (bFromSweep :type Boolean) (SweepResult :type Hit%20Result%20Structure%20%28by%20ref%29))
  ;[0.15 0.15 0.15 0.5] Texte pour prendre les plats
  (Rendering|SetVisibility (Variables|Default|GetTexte%20F) true false))

(event OnComponentEndOverlap(Box)
  (params (OverlappedComponent :type Primitive%20Component%20Object%20Reference) (OtherActor :type Actor%20Object%20Reference) (OtherComp :type Primitive%20Component%20Object%20Reference) (OtherBodyIndex :type Integer))
  ;[0.15 0.15 0.15 0.5] Texte pour prendre les plats
  (Rendering|SetVisibility (Variables|Default|GetTexte%20F) false false))

(event EventBeginPlay
  ;[0.15 0.15 0.15 0.5] Keyboard qui marche
  (Input|EnableInput (Game|GetPlayerController 0)))

(event Input|KeyboardEvents|F
  (params (Key :type Key%20Structure :default "None"))
  ;[0.15 0.15 0.15 0.5] Presser F pour détruire plats
  (:Pressed
    (if (Collision|IsOverlappingActor (Variables|Default|GetBox) (Game|Player|GetPlayerPawn 0) :!class /Script/Engine.PrimitiveComponent)
      (bind _asbp_main_chara (Utilities|Casting|CastToBP_MainChara (Game|Player|GetPlayerPawn 0)))
      (Default|AjoutPlat _asbp_main_chara)
      (Actor|DestroyActor))))

(fn ConstructionScript)